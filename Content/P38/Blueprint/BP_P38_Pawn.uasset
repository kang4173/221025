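; Player-controlled P-38 aircraft pawn that flies forward constantly and fires rockets.
; Tick spins both propellers and feeds the actor's forward vector into FloatingPawnMovement, so steering only rotates the actor: Right axis rolls, Forward axis pitches.
; Fire spawns BP_Rocket at the Arrow component's transform.
; Holding Left Shift boosts by raising the movement component's MaxSpeed, restored to a fixed slower speed on release.
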(event `self.ReceiveTick`
  (params (DeltaSeconds :type "Float (single-precision)"))
  ;[1 1 1] P-38 Propeller Speed
  ;;[1 1 1] Left
  (`SceneComponent.K2_AddLocalRotation` (`self.Left`) (`KismetMathLibrary.MakeRotator` (* (`self.PropellerSpeed`) (`GameplayStatics.GetWorldDeltaSeconds`))) false false)
  ;;[1 1 1] Right
  (`SceneComponent.K2_AddLocalRotation` (`self.Right`) (`KismetMathLibrary.MakeRotator` (* (`self.PropellerSpeed`) (`GameplayStatics.GetWorldDeltaSeconds`))) false false)
  ;[1 1 1] Floa~Movement 사용
  (`self.AddMovementInput` (`self.GetActorForwardVector`)))

(event `InputAxis|Right`
  (params (AxisValue :type "Float (single-precision)"))
  ;[1 1 1] Move
  ;;[1 1 1] Move Forward (Roll)
  (`self.K2_AddActorLocalRotation` (`KismetMathLibrary.MakeRotator` (* (`KismetMathLibrary.FClamp` AxisValue -1.0) (`self.RotationSpeed`) (`GameplayStatics.GetWorldDeltaSeconds`)))))

(event `InputAxis|Forward`
  (params (AxisValue :type "Float (single-precision)"))
  ;[1 1 1] Move
  ;;[1 1 1] Move Right(pitch)
  (`self.K2_AddActorLocalRotation` (`KismetMathLibrary.MakeRotator` 0.0 (* (`KismetMathLibrary.FClamp` AxisValue -1.0) (`self.RotationSpeed`) (`GameplayStatics.GetWorldDeltaSeconds`)))))

(event `InputAction|Fire`
  (params (Key :type "Key Structure"))
  ;[1 1 1] Rocket
  (:`Pressed`
    (`|SpawnActorFromClass` "/Game/P38/Blueprint/BP_Rocket.BP_Rocket_C" (`SceneComponent.K2_GetComponentToWorld` (`self.Arrow`)) "Undefined" "OverrideRootScale" null null)))

(event `Key|LeftShift`
  (params (Key :type "Key Structure"))
  ;[1 1 1] Booster
  (:`Pressed`
    (bind _output_get (set `self.P38Speed` 800.0))
    (set `FloatingPawnMovement.MaxSpeed` _output_get (`self.FloatingPawnMovement`)))
  (:`Released`
    (bind _output_get_2 (set `self.P38Speed` 50.0))
    (set `FloatingPawnMovement.MaxSpeed` _output_get_2 (`self.FloatingPawnMovement`))))

(fn `UserConstructionScript`)