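; BP_P38 is a P-38 aircraft Blueprint with spinning propellers and input-driven rotation.
; Tick rolls the Left and Right components at PropellerSpeed, scaled by delta time.
; The Forward axis rolls the actor at RotationSpeed, while the Right axis is meant for pitch but multiplies by zero, so it has no effect.
; A forward offset of Body by P38Speed is present but unconnected, so it never runs.
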(event `self.ReceiveTick`
  (params (DeltaSeconds :type "Float (single-precision)"))
  ;[1 1 1] P-38 Propeller Speed
  ;;[1 1 1] Left
  (`SceneComponent.K2_AddLocalRotation` (`self.Left`) (`KismetMathLibrary.MakeRotator` (* (`self.PropellerSpeed`) (`GameplayStatics.GetWorldDeltaSeconds`))) false false)
  ;;[1 1 1] Right
  (`SceneComponent.K2_AddLocalRotation` (`self.Right`) (`KismetMathLibrary.MakeRotator` (* (`self.PropellerSpeed`) (`GameplayStatics.GetWorldDeltaSeconds`))) false false))

(event `InputAxis|Forward`
  (params (AxisValue :type "Float (single-precision)"))
  ;[1 1 1] Move
  ;;[1 1 1] Move Forward (Roll)
  (`self.K2_AddActorLocalRotation` (`KismetMathLibrary.MakeRotator` (* AxisValue (`self.RotationSpeed`) (`GameplayStatics.GetWorldDeltaSeconds`)))))

(event `InputAxis|Right`
  (params (AxisValue :type "Float (single-precision)"))
  ;[1 1 1] Move
  ;;[1 1 1] Move Right(pitch)
  (`self.K2_AddActorLocalRotation` (`KismetMathLibrary.MakeRotator` 0.0 (* 0.0 (`self.RotationSpeed`) (`GameplayStatics.GetWorldDeltaSeconds`)))))

(fn `UserConstructionScript`)